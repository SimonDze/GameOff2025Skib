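; BP_Object is a pickup object that highlights itself when the third-person character comes within range.
; Begin and end overlap events filtered to that character toggle a white outline overlay material on the Sphere, print debug messages and notify OverlayComponent of range entry or exit.
; The PickUp function hides the actor and destroys its root, collision box and sphere components, rather than destroying the actor itself.
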(event `self.ReceiveBeginPlay`
  (`MeshComponent.SetOverlayMaterial` (`self.Sphere`) null))

(event `self.ReceiveActorBeginOverlap`
  (params (OtherActor :type "Actor Object Reference"))
  (cast `/Game/ThirdPerson/Blueprints/BP_ThirdPersonCharacter` OtherActor)
  (`MeshComponent.SetOverlayMaterial` (`self.Sphere`) "/Game/Materials/m_outlineWhite.m_outlineWhite")
  (`KismetSystemLibrary.PrintString` "Hello")
  (`/Game/ActorComponent/OverlayComponent.onPlayerEnterRange` (`self.OverlayComponent`)))

(event `self.ReceiveActorEndOverlap`
  (params (OtherActor :type "Actor Object Reference"))
  (cast `/Game/ThirdPerson/Blueprints/BP_ThirdPersonCharacter` OtherActor)
  (`MeshComponent.SetOverlayMaterial` (`self.Sphere`) null)
  (`KismetSystemLibrary.PrintString` "Bye")
  (`/Game/ActorComponent/OverlayComponent.onPlayerExitRange` (`self.OverlayComponent`)))

(fn `PickUp`
  (`self.SetActorHiddenInGame` true)
  (`ActorComponent.K2_DestroyComponent` (`self.DefaultSceneRoot`))
  (`ActorComponent.K2_DestroyComponent` (`self.BoxCollision`))
  (`ActorComponent.K2_DestroyComponent` (`self.Sphere`)))

(fn `UserConstructionScript`)