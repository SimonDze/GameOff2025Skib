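; BP_RandomSpawner is an actor that spawns a randomized BP_Object at its own transform when play begins.
; It passes food, water, wood, rope and sail values, plus a texture and mesh, to the new object's InitValuees.
; These properties are read from the Objects array using random index lookups, and the spawn adjusts for collisions but always succeeds.
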(event `self.ReceiveBeginPlay`
  (bind _output (`|GetArrayItem` (`self.Objects`) (`KismetMathLibrary.RandomIntegerInRange` 0 (- (`KismetArrayLibrary.Array_Length` (`self.Objects`)) 1))))
  (bind _returnvalue (`|SpawnActorFromClass` "/Game/Blueprints/BP_Object.BP_Object_C" (`self.GetTransform`) "AdjustIfPossibleButAlwaysSpawn" "MultiplyWithRoot" null null 0 0 null))
  (`/Game/Blueprints/BP_Object.InitValuees` _returnvalue (`/Game/Blueprints/BP_Object.FoodValue` _output) (`/Game/Blueprints/BP_Object.WaterValue` _output) (`/Game/Blueprints/BP_Object.objectTexture` _output) (`/Game/Blueprints/BP_Object.mesh` _output) (`/Game/Blueprints/BP_Object.WoodValue` _output) (`/Game/Blueprints/BP_Object.RopeValue` _output) (`/Game/Blueprints/BP_Object.SailValue` _output)))

(fn `UserConstructionScript`)