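; BP_Object is a collectible item actor that carries a mesh, a texture and food, water, wood, rope and sail values, set through InitValuees.
; When BP_ThirdPersonCharacter overlaps it with inventory space left, it applies a white outline overlay material and notifies its OverlayComponent.
; Ending the overlap clears the outline and notifies the component of the exit.
; PickUp hides the actor and destroys its components rather than the actor itself.
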(event `self.ReceiveActorBeginOverlap`
  (params (OtherActor :type "Actor Object Reference"))
  (bind _asbp_third_person_character (cast `/Game/ThirdPerson/Blueprints/BP_ThirdPersonCharacter` OtherActor))
  (if (< (`KismetArrayLibrary.Array_Length` (`/Game/ThirdPerson/Blueprints/BP_ThirdPersonCharacter.itemsInInventory` _asbp_third_person_character)) (`/Game/ThirdPerson/Blueprints/BP_ThirdPersonCharacter.maxItemInInventory` _asbp_third_person_character))
    (`MeshComponent.SetOverlayMaterial` (`self.Sphere`) "/Game/Materials/m_outlineWhite.m_outlineWhite")
    (`KismetSystemLibrary.PrintString` "Hello")
    (`/Game/ActorComponent/OverlayComponent.onPlayerEnterRange` (`self.OverlayComponent`))))

(event `self.ReceiveActorEndOverlap`
  (params (OtherActor :type "Actor Object Reference"))
  (cast `/Game/ThirdPerson/Blueprints/BP_ThirdPersonCharacter` OtherActor)
  (`MeshComponent.SetOverlayMaterial` (`self.Sphere`) null)
  (`KismetSystemLibrary.PrintString` "Bye")
  (`/Game/ActorComponent/OverlayComponent.onPlayerExitRange` (`self.OverlayComponent`)))

(fn `InitValuees`
  (params (food :type Integer) (water :type Integer) (texture :type "Texture2D Object Reference") (mesh :type "StaticMesh Object Reference") (wood :type Integer) (Rope :type Integer) (sail :type Integer))
  (`StaticMeshComponent.SetStaticMesh` (`self.Sphere`) mesh)
  (`MeshComponent.SetOverlayMaterial` (`self.Sphere`) null)
  (set `self.FoodValue` food)
  (set `self.WaterValue` water)
  (set `self.objectTexture` texture)
  (set `self.WoodValue` wood)
  (set `self.RopeValue` Rope)
  (set `self.SailValue` sail))

(fn `PickUp`
  (`self.SetActorHiddenInGame` true)
  (`ActorComponent.K2_DestroyComponent` (`self.DefaultSceneRoot`))
  (`ActorComponent.K2_DestroyComponent` (`self.BoxCollision`))
  (`ActorComponent.K2_DestroyComponent` (`self.Sphere`)))

(fn `UserConstructionScript`
  (`StaticMeshComponent.SetStaticMesh` (`self.Sphere`) (`self.mesh`))
  (`MeshComponent.SetOverlayMaterial` (`self.Sphere`) null))