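; BP_DepositZone is a zone actor that reacts when the player character enters or leaves it.
; On overlap with BP_ThirdPersonCharacter, it applies a white outline overlay material to its Cylinder and clears it on exit.
; It notifies its OverlayComponent of player enter and exit range and prints debug greetings.
; No deposit logic exists in its graphs.
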(event `self.ReceiveActorBeginOverlap`
  (params (OtherActor :type "Actor Object Reference"))
  (cast `/Game/ThirdPerson/Blueprints/BP_ThirdPersonCharacter` OtherActor)
  (`MeshComponent.SetOverlayMaterial` (`self.Cylinder`) "/Game/Materials/m_outlineWhite.m_outlineWhite")
  (`KismetSystemLibrary.PrintString` "Hello")
  (`/Game/ActorComponent/OverlayComponent.onPlayerEnterRange` (`self.OverlayComponent`)))

(event `self.ReceiveActorEndOverlap`
  (params (OtherActor :type "Actor Object Reference"))
  (cast `/Game/ThirdPerson/Blueprints/BP_ThirdPersonCharacter` OtherActor)
  (`MeshComponent.SetOverlayMaterial` (`self.Cylinder`) null)
  (`KismetSystemLibrary.PrintString` "Bye")
  (`/Game/ActorComponent/OverlayComponent.onPlayerExitRange` (`self.OverlayComponent`)))

(fn `UserConstructionScript`)